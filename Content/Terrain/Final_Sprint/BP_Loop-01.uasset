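; Loop terrain piece for the Final Sprint level set, with a trigger volume that detects the player pawn leaving it.
; On end overlap it prints a yellow debug message naming the piece.
; If CreateTileOnEndOverlap is set it then casts the game instance to GGJGameInstance, but nothing follows the cast, so no tile is created here.
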(event `self.ReceiveBeginPlay`)

(event `self.TriggerVolume.OnComponentEndOverlap`
  (params (OverlappedComponent :type "PrimitiveComponent Object Reference") (OtherActor :type "Actor Object Reference") (OtherComp :type "PrimitiveComponent Object Reference") (OtherBodyIndex :type Integer))
  (if (== OtherActor (`GameplayStatics.GetPlayerPawn` 0))
    (`KismetSystemLibrary.PrintString` (`KismetStringLibrary.Concat_StrStr` "Loop " (`KismetSystemLibrary.GetDisplayName` self)) true true (struct :`R` 1.0 :`G` 0.908244 :`B` 0.181247 :`A` 1.0))
    (if (`self.CreateTileOnEndOverlap`)
      (cast `/Game/Level/GGJGameInstance` (`GameplayStatics.GetGameInstance`)))))

(fn `UserConstructionScript`)